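; Player hero character that moves camera-relative, dashes, forwards attack and skill input to cycled weapons, creates the HUD and quits the game on death.
; Dash applies an impulse, trail and temporary collision-channel change under a cooldown timer.
; While attacking, stick input steers rotation, with optional cone auto-aim that holds the last target.
; Rage charges a timed berserk that swaps mesh, speed, damage taken and dash cooldown, and notifies weapons via BPI_HeroWeapon.
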(event `InputAction|Dash`
  (params (Key :type "Key Structure"))
  (bind (_returnvalue_roll _returnvalue_pitch _returnvalue_yaw) (`KismetMathLibrary.BreakRotator` (`SceneComponent.K2_GetComponentRotation` (`self.Camera`))))
  (bind _direction (`self.DirectionVector` (`self.ForwardAxisInput`) (`self.RightAxisInput`) _returnvalue_yaw))
  ;[1 1 1] Dash
  (:`Pressed`
    (if (`self.DashNotOnCooldown`)
      (`/Game/MicroDoom/Weapons/BP_BaseWeapon.InterruptAction` (`self.GetCurrentWeapon`))
      (`self.SetDashingState` true)
      (`ParticleSystemComponent.BeginTrails` (`self.DashTrail`) "FX_DashTrail_1" "FX_DashTrail_2" "ETrailWidthMode_FromFirst" 1.0)
      (`CharacterMovementComponent.AddImpulse` (`self.CharacterMovement`) (* (`KismetMathLibrary.Normal` (`KismetMathLibrary.SelectVector` (`KismetMathLibrary.Conv_RotatorToVector` (`SceneComponent.K2_GetComponentRotation` (`self.CapsuleComponent`))) _direction (== _direction (0.0 0.0 0.0)))) (`self.DashPower`)) true)
      (`KismetSystemLibrary.K2_SetTimerDelegate` (delegate `ReturnCollision`) (`self.NoCollisionDuration`))
      (bind _returnvalue (`KismetSystemLibrary.K2_SetTimerDelegate` (delegate `OnStopDash`) (`self.DashCoolDown`)))
      (set `self.DashCooldownTimer` _returnvalue))))

(event `ReturnCollision`
  ;[1 1 1] Dash
  (`self.SetDashingState` false)
  (`ParticleSystemComponent.EndTrails` (`self.DashTrail`)))

(event `OnStopDash`
  ;[1 1 1] Dash
)

(event `InputAxis|MoveForward`
  (params (AxisValue :type "Float (single-precision)"))
  (bind (_returnvalue_roll _returnvalue_pitch _returnvalue_yaw) (`KismetMathLibrary.BreakRotator` (`SceneComponent.K2_GetComponentRotation` (`self.Camera`))))
  ;[1 1 1] Movement
  (bind _output_get (set `self.ForwardAxisInput` AxisValue))
  (`self.ControllHeroMovement` _returnvalue_yaw _output_get true))

(event `self.ReceiveTick`
  (params (DeltaSeconds :type "Float (single-precision)"))
  (bind (_returnvalue_roll _returnvalue_pitch _returnvalue_yaw) (`KismetMathLibrary.BreakRotator` (`SceneComponent.K2_GetComponentRotation` (`self.Camera`))))
  (`parent.ReceiveTick` DeltaSeconds)
  ;[1 1 1] Movement
  (`self.ControllHeroAttackRotation` _returnvalue_yaw (`self.ForwardAxisInput`) (`self.RightAxisInput`)))

(event `InputAxis|MoveRight`
  (params (AxisValue :type "Float (single-precision)"))
  (bind (_returnvalue_roll _returnvalue_pitch _returnvalue_yaw) (`KismetMathLibrary.BreakRotator` (`SceneComponent.K2_GetComponentRotation` (`self.Camera`))))
  ;[1 1 1] Movement
  (bind _output_get (set `self.RightAxisInput` AxisValue))
  (`self.ControllHeroMovement` _returnvalue_yaw _output_get))

(event `InputAction|Attack`
  (params (Key :type "Key Structure"))
  (bind _weapon (`self.GetCurrentWeapon`))
  ;[1 1 1] Combat
  (:`Pressed`
    (`/Game/MicroDoom/Weapons/BP_BaseWeapon.CallMainAttack` _weapon null))
  (:`Released`
    (`/Game/MicroDoom/Weapons/BP_BaseWeapon.AttackRelease` _weapon :!label _label)))

(event `InputAction|Skill`
  (params (Key :type "Key Structure"))
  ;[1 1 1] Combat
  (:`Pressed`
    (`/Game/MicroDoom/Weapons/BP_BaseWeapon.CallSpecial` (`self.GetCurrentWeapon`)))
  (:`Released`
    (goto _label)))

(event `InputAction|ChoosePrevWeapon`
  (params (Key :type "Key Structure"))
  (bind _returnvalue (- (`self.CurrentWeaponNum`) 1))
  ;[1 1 1] Changing weapon
  (:`Pressed`
    (`self.ChangeWeapon` (`KismetMathLibrary.SelectInt` (- (`KismetArrayLibrary.Array_Length` (`self.WeaponInstances`)) 1) _returnvalue (< _returnvalue 0)))))

(event `InputAction|ChooseNextWeapon`
  (params (Key :type "Key Structure"))
  (bind _returnvalue (+ (`self.CurrentWeaponNum`) 1))
  ;[1 1 1] Changing weapon
  (:`Pressed`
    (`self.ChangeWeapon` (`KismetMathLibrary.SelectInt` 0 _returnvalue (== _returnvalue (`KismetArrayLibrary.Array_Length` (`self.WeaponInstances`)))))))

(event `InputAction|BercerkOn`
  (params (Key :type "Key Structure"))
  (:`Pressed`
    (if (and (not (`self.BercerkOnCooldown`)) (not (`self.bBercerk`)))
      (`self.BercerkOn`)
      (`KismetSystemLibrary.K2_SetTimerDelegate` (delegate `SwitchOffBercerk`) (`self.BercerkDuration`)))))

(event `SwitchOffBercerk`
  (`self.BercerkOff`))

(event `/Game/MicroDoom/Util/BPI_Ragable.AddRage`
  (params (Amount :type "Float (single-precision)"))
  (`self.UpdateBercerkCooldown` Amount))

(event `self.ReceiveBeginPlay`
  (`parent.ReceiveBeginPlay`)
  (`self.SetupHud`)
  (`self.SetBercerkCooldown` true))

(event `/Game/MicroDoom/Util/BPI_CanAutoAim.SetAutoAimingParameters`
  (params (AutoAimingDegrees :type "Float (single-precision)") (AutoAimingRange :type "Float (single-precision)") (AutoAimingStopFollowDegrees :type "Float (single-precision)"))
  (set `self.bAutoAiming` true)
  (set `self.AutoAimingDegrees` AutoAimingDegrees)
  (set `self.Range` AutoAimingRange)
  (set `self.StopFollowTargetDegrees` AutoAimingStopFollowDegrees))

(event `/Game/MicroDoom/Util/BPI_CanAutoAim.ResetAutoAiming`
  (set `self.bAutoAiming` false))

(fn `BercerkOff`
  (bind _charactermovement (`self.CharacterMovement`))
  ;[1 1 1] Reset mesh
  (`SkinnedMeshComponent.SetSkinnedAssetAndUpdate` (`self.Mesh`) (`self.SavedMesh`) true)
  ;[1 1 1] Reset walk speed
  (set `CharacterMovementComponent.MaxWalkSpeed` (/ (`CharacterMovementComponent.MaxWalkSpeed` _charactermovement) (`self.BerserkSpeedMul`)) _charactermovement)
  ;[1 1 1] Reset berserk for weapons
  (for _array_element (`self.WeaponInstances`)
    (if (`KismetSystemLibrary.DoesImplementInterface` _array_element "/Game/MicroDoom/Util/BPI_HeroWeapon.BPI_HeroWeapon_C")
      (`/Game/MicroDoom/Util/BPI_HeroWeapon.BercerkOff` _array_element)
      ;[1 1 1] Reset gotten dmg multiplier
      (set `self.GottenDmgMultiplier` (`self.SavedGottenDamageMultipier`))
      ;[1 1 1] ResetDash cooldown
      (set `self.DashCoolDown` (`self.SavedDashCooldown`))
      (set `self.bBercerk` false))))

(fn `BercerkOn`
  (bind _charactermovement (`self.CharacterMovement`))
  (`self.SetBercerkCooldown` true)
  (set `self.bBercerk` true)
  ;[1 1 1] Save old mesh
  (set `self.SavedMesh` (`SkinnedMeshComponent.SkeletalMesh` (`self.Mesh`)))
  ;[1 1 1] Set new mesh
  (`SkinnedMeshComponent.SetSkinnedAssetAndUpdate` (`self.Mesh`) (`self.BerserkMesh`) true)
  ;[1 1 1] Set new speed
  (set `CharacterMovementComponent.MaxWalkSpeed` (* (`CharacterMovementComponent.MaxWalkSpeed` _charactermovement) (`self.BerserkSpeedMul`)) _charactermovement)
  ;[1 1 1] Call bercerk on all weapons
  (for _array_element (`self.WeaponInstances`)
    (if (`KismetSystemLibrary.DoesImplementInterface` _array_element "/Game/MicroDoom/Util/BPI_HeroWeapon.BPI_HeroWeapon_C")
      (`/Game/MicroDoom/Util/BPI_HeroWeapon.BercerkOn` _array_element)))
  ;[1 1 1] Save dmg multiplier
  (set `self.SavedGottenDamageMultipier` (`self.GottenDmgMultiplier`))
  ;[1 1 1] Set new damage multiplier
  (set `self.GottenDmgMultiplier` (`self.BercerkGottenDamageMultiplier`))
  ;[1 1 1] Save dash cooldown
  (set `self.SavedDashCooldown` (`self.DashCoolDown`))
  ;[1 1 1] Set new dash cooldown
  (set `self.DashCoolDown` (`self.BercerkDashCoolDown`)))

(fn `ControllHeroAttackRotation`
  (params (CameraYaw :type "Float (double-precision)") (ForwardAxis :type "Float (double-precision)") (RightAxis :type "Float (double-precision)"))
  (locals (CurrentRotationInput :type "Rotator Structure" :default (struct)) (bHasAimInThisFrame :type Boolean) (bHasAimFromLastFrame :type Boolean) (bHoldStick :type Boolean) (CurrentFoundAim :type "Actor Object Reference") (bLastTargetIsCloseToRotation :type Boolean))
  (bind _bhasaiminthisframe (`local.bHasAimInThisFrame`))
  (bind _bhasaimfromlastframe (`local.bHasAimFromLastFrame`))
  ;[1 1 1] Rotate only while attacking
  (if (`self.bAttacking`)
    ;[1 1 1] Get rotation vector relative ro camera yaw
    (set `local.CurrentRotationInput` (`KismetMathLibrary.Conv_VectorToRotator` (`self.DirectionVector` ForwardAxis RightAxis CameraYaw)))
    ;[1 1 1] Was any rotation input in current frame?
    (set `local.bHoldStick` (not (== (`local.CurrentRotationInput`) (struct))))
    (if (not (`local.bHoldStick`))
      (set `local.CurrentRotationInput` (`self.K2_GetActorRotation`)))
    (if (`self.bAutoAiming`)
      ;[1 1 1] Autoaim
      ;;[1 1 1] Get state flags
      (bind _closesttarget (`/Game/MicroDoom/Util/ConeDetectionUtil.FindTargetInCone` (`local.CurrentRotationInput`) (`self.AutoAimingDegrees`) "Enemy" self (`self.Range`)))
      (bind _output_get (set `local.CurrentFoundAim` _closesttarget))
      (set `local.bHasAimInThisFrame` (`KismetSystemLibrary.IsValid` _output_get))
      (bind _output_get_2 (set `local.bHasAimFromLastFrame` (`KismetSystemLibrary.IsValid` (`self.LastAimTarget`))))
      (if _output_get_2
        (set `local.bLastTargetIsCloseToRotation` (< (`KismetMathLibrary.Abs` (`/Game/MicroDoom/Util/ConeDetectionUtil.CalculateDegreeDiff` (`self.LastAimTarget`) self (`local.CurrentRotationInput`))) (`self.StopFollowTargetDegrees`)))
        (else
          (set `local.bLastTargetIsCloseToRotation` false)))
      ;;[1 1 1] Check conditions
      (if (`local.bHoldStick`)
        (if _bhasaiminthisframe
          ;;[1 1 1] Set rototion to new found target and save it
          (`self.K2_SetActorRotation` (`KismetMathLibrary.MakeRotator` 0.0 0.0 (`/Game/MicroDoom/Util/ConeDetectionUtil.RotationToActor` self (`local.CurrentFoundAim`))) :!label _label)
          (set `self.LastAimTarget` (`local.CurrentFoundAim`))
          (elif (`local.bLastTargetIsCloseToRotation`)
            ;;[1 1 1] Set rotation to last target
            (`self.K2_SetActorRotation` (`KismetMathLibrary.MakeRotator` 0.0 0.0 (`/Game/MicroDoom/Util/ConeDetectionUtil.RotationToActor` self (`self.LastAimTarget`))) :!label _label_2)
            (else
              ;;[1 1 1] Reset last aim target and rotaion according to input
              (set `self.LastAimTarget` null)
              (`self.K2_SetActorRotation` (`KismetMathLibrary.RInterpTo` (`SceneComponent.K2_GetComponentRotation` (`self.CapsuleComponent`)) (`local.CurrentRotationInput`) (`GameplayStatics.GetWorldDeltaSeconds`) (`/Game/MicroDoom/Weapons/BP_BaseWeapon.HeroRotationSpeed` (`self.GetCurrentWeapon`))) :!label _label_3))))
        (elif _bhasaiminthisframe
          (if _bhasaimfromlastframe
            (goto _label_2)
            (else
              (goto _label)))
          (elif _bhasaimfromlastframe
            (goto _label_2)
            (else
              ;;[1 1 1] Reset last aim target and do nothing
              (set `self.LastAimTarget` null)))))
      (else
        (goto _label_3)))
    (else
      (set `self.LastAimTarget` null))))

(fn `ControllHeroMovement`
  (params (CameraYaw :type "Float (double-precision)") (AxisValue :type "Float (double-precision)") (bForward :type Boolean))
  (locals (RoundedAxisValue :type "Float (double-precision)"))
  (if (`self.bMoving`)
    ;[1 1 1] Round axis value
    (if (< AxisValue 0.0)
      (set `local.RoundedAxisValue` -1.0)
      (elif (> AxisValue 0.0)
        (set `local.RoundedAxisValue` 1.0)
        (else
          (set `local.RoundedAxisValue` 0.0))))
    (`self.AddMovementInput` (`KismetMathLibrary.RotateAngleAxis` (`KismetMathLibrary.SelectVector` (1.0 0.0 0.0) (0.0 1.0 0.0) bForward) CameraYaw (0.0 0.0 1.0)) (`local.RoundedAxisValue`))))

(fn `Die`
  (params (Killer :type "Actor Object Reference"))
  (`parent.Die` Killer)
  (`KismetSystemLibrary.QuitGame` null "Quit"))

(fn `GetBercerkCooldownFraction`
  (returns (CooldownFraction :type "Float (double-precision)"))
  (return (/ (`self.BercerkCurrentCooldown`) (`self.BercerkCooldown`))))

(fn `GetDashCoolDownPercent`
  (returns (CoolDownPercent :type "Float (double-precision)"))
  (return (/ (- (`self.DashCoolDown`) (`KismetSystemLibrary.K2_GetTimerRemainingTimeHandle` (`self.DashCooldownTimer`))) (`self.DashCoolDown`))))

(fn `HandleDmg`
  (params (DamageCauser :type "Actor Object Reference"))
  (`parent.HandleDmg` null)
  (bind _returnvalue (`|CreateWidget` "/Game/MicroDoom/UI/BP_HeroDmgPopUp.BP_HeroDmgPopUp_C" null (`KismetMathLibrary.FTrunc` (`self.GottenDmg`)) (- (`GameplayStatics.ProjectWorldToScreen` (`GameplayStatics.GetPlayerController` 0) (`SceneComponent.K2_GetComponentLocation` (`self.CapsuleComponent`))) (64.0 16.0))))
  (`UserWidget.AddToViewport` _returnvalue 0))

(fn `IsInRage`
  (returns (IsInRage :type Boolean))
  (return (`self.bBercerk`)))

(fn `QuitOnDie`)

(fn `SetBercerkCooldown`
  (params (Cooldown :type Boolean))
  (bind _output_get (set `self.BercerkOnCooldown` Cooldown))
  (set `self.BercerkCurrentCooldown` (`KismetMathLibrary.SelectFloat` 0.0 (`self.BercerkCooldown`) _output_get)))

(fn `SetDashingState`
  (params (bDashing :type Boolean))
  (`PrimitiveComponent.SetCollisionObjectType` (`self.CapsuleComponent`) (select `bool` bDashing :`false` "ECC_Pawn" :`true` "ECC_GameTraceChannel1" :!type "ECollisionChannel Enum")))

(fn `SetupHud`
  (bind _returnvalue (`|CreateWidget` "/Game/MicroDoom/UI/BP_HUD.BP_HUD_C"))
  (`UserWidget.AddToPlayerScreen` _returnvalue 0))

(fn `UpdateBercerkCooldown`
  (params (Change :type "Float (double-precision)"))
  (if (`self.BercerkOnCooldown`)
    (bind _output_get (set `self.BercerkCurrentCooldown` (`KismetMathLibrary.FClamp` (+ Change (`self.BercerkCurrentCooldown`)) 0.0 (`self.BercerkCooldown`))))
    (set `self.BercerkOnCooldown` (!= _output_get (`self.BercerkCooldown`)))))

(fn `UserConstructionScript`
  (`parent.UserConstructionScript`))