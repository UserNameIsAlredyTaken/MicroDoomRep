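; Base enemy character that handles damage feedback, collision damage and collectable drops on death.
; Its health bar widget updates every tick, while hits taken spawn a screen-projected damage popup, fiery particles and a material flash.
; With PushDamage on, collisions with damage-on-hit actors damage both sides, throttled by a timer-reset DoOnce.
; Death drops healing if the player is raging, otherwise rage when EffectedBySword and the killer isn't a hero weapon.
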(event `self.ReceiveBeginPlay`
  (`parent.ReceiveBeginPlay`)
  (bind _asbp_enemy_health (cast `/Game/MicroDoom/UI/BP_EnemyHealth` (`WidgetComponent.GetUserWidgetObject` (`self.HealthBar`))))
  (`/Game/MicroDoom/UI/BP_EnemyHealth.SetOwnerEnemy` _asbp_enemy_health self))

(event `self.ReceiveTick`
  (params (DeltaSeconds :type "Float (single-precision)"))
  (`parent.ReceiveTick` DeltaSeconds)
  (`self.UpdateHealtBar`))

(event `self.ReceiveHit`
  (params (MyComp :type "PrimitiveComponent Object Reference") (Other :type "Actor Object Reference") (OtherComp :type "PrimitiveComponent Object Reference") (bSelfMoved :type Boolean) (HitLocation :type "Vector Structure") (HitNormal :type "Vector Structure") (NormalImpulse :type "Vector Structure") (Hit :type "HitResult Structure (by ref)"))
  (set `self.OtherHitter` Other)
  (if (`KismetSystemLibrary.DoesImplementInterface` Other "/Game/MicroDoom/Util/BPI_ApplyDamageOnHit.BPI_ApplyDamageOnHit_C")
    (if (`self.PushDamage`)
      (`/Engine/EditorBlueprintResources/StandardMacros.DoOnce` false :!label _label
        (:`Completed`
          (bind _damage (message `/Game/MicroDoom/Util/BPI_ApplyDamageOnHit.GetHitDamage` (`self.OtherHitter`)))
          (bind _damage_2 (message `/Game/MicroDoom/Util/BPI_ApplyDamageOnHit.GetHitDamage` self))
          (`GameplayStatics.ApplyDamage` self _damage null (`self.OtherHitter`))
          (`GameplayStatics.ApplyDamage` (`self.OtherHitter`) _damage_2 null self)
          (`KismetSystemLibrary.K2_SetTimerDelegate` (delegate `ResetDelay`) (`self.HitDelay`)))))))

(event `ResetDelay`
  (goto _label :!via `Reset`))

(event `ChangeColor`
  (bind _returnvalue (`MeshComponent.GetMaterials` (`self.Mesh`)))
  (set `self.OldMat` _returnvalue)
  (for (_ _array_index) _returnvalue
    (`PrimitiveComponent.SetMaterial` (`self.Mesh`) _array_index (`self.DmgMat`))
    (`KismetSystemLibrary.Delay` 0.12)
    (for (_array_element _array_index_2) (`self.OldMat`)
      (`PrimitiveComponent.SetMaterial` (`self.Mesh`) _array_index_2 _array_element))))

(fn `CharHandleDmg`
  (params (DamageCauser :type "Actor Object Reference"))
  (bind (_returnvalue_roll _returnvalue_pitch _returnvalue_yaw) (`KismetMathLibrary.BreakRotator` (`KismetMathLibrary.Conv_VectorToRotator` (- (`self.K2_GetActorLocation`) (`self.K2_GetActorLocation` DamageCauser)))))
  (`parent.CharHandleDmg` null)
  (bind _returnvalue (`|CreateWidget` "/Game/MicroDoom/UI/EnemyDmgPopUp.EnemyDmgPopUp_C" null (`KismetMathLibrary.FTrunc` (`self.GottenDmg`)) (- (`GameplayStatics.ProjectWorldToScreen` (`GameplayStatics.GetPlayerController` 0) (`SceneComponent.K2_GetComponentLocation` (`self.CapsuleComponent`))) (64.0 16.0))))
  (`UserWidget.AddToViewport` _returnvalue 0)
  (`self.ChangeColor`)
  ;[1 1 1] Spawn FX
  (`GameplayStatics.SpawnEmitterAtLocation` "/Game/P_ForgeDip_Firey.P_ForgeDip_Firey" (`SceneComponent.K2_GetComponentLocation` (`self.CapsuleComponent`)) (`KismetMathLibrary.MakeRotator` 0.0 0.0 _returnvalue_yaw) (3.0 3.0 3.0)))

(fn `Die`
  (params (Killer :type "Actor Object Reference"))
  (bind _returnvalue (`GameplayStatics.GetPlayerPawn` 0))
  (`parent.Die` Killer)
  ;[1 1 1] If player in bercerk mode, leave health
  (if (`KismetSystemLibrary.DoesImplementInterface` _returnvalue "/Game/MicroDoom/Util/BPI_Ragable.BPI_Ragable_C")
    (bind _isinrage (message `/Game/MicroDoom/Util/BPI_Ragable.IsInRage` _returnvalue))
    (if _isinrage
      (`|SpawnActorFromClass` "/Game/MicroDoom/Objects/Collectables/BP_HealCollectable.BP_HealCollectable_C" (`self.SlightlyRandomSpawnLocation`) "Undefined" "OverrideRootScale" null null)
      (else
        ;[1 1 1] If died not from weapon leave rage
        (if (and (not (`KismetSystemLibrary.DoesImplementInterface` Killer "/Game/MicroDoom/Util/BPI_HeroWeapon.BPI_HeroWeapon_C")) (`self.bEffectedBySword`))
          (`|SpawnActorFromClass` "/Game/MicroDoom/Objects/Collectables/BP_RageCollectable.BP_RageCollectable_C" (`self.SlightlyRandomSpawnLocation`) "Undefined" "OverrideRootScale" null null))))))

(fn `GetHitDamage`
  (returns (Damage :type "Float (double-precision)"))
  (return (`self.HitDamage`)))

(fn `GetPushDamageOn`
  (returns (bPushDamage :type Boolean))
  (return (`self.PushDamage`)))

(fn `UpdateHealtBar`
  (bind _asbp_enemy_health (cast `/Game/MicroDoom/UI/BP_EnemyHealth` (`WidgetComponent.GetUserWidgetObject` (`self.HealthBar`))))
  (`ProgressBar.SetPercent` (`/Game/MicroDoom/UI/BP_EnemyHealth.ProgressBar_13` _asbp_enemy_health) (/ (`self.CurrentHealth`) (`self.MaxHealth`))))

(fn `UserConstructionScript`
  (`parent.UserConstructionScript`))