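; Base character for MicroDoom that handles health, death, weapons and knockback.
; On BeginPlay it spawns every weapon class, attaches each to a mesh socket and activates only one; switching is blocked while attacking.
; Damage reduces clamped health unless invincible; death destroys attached actors in reverse order, then the character.
; Push applies an impulse and stuns by unpossessing the AI controller, which a timer repossesses.
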(event `self.ReceiveAnyDamage`
  (params (Damage :type "Float (single-precision)") (DamageType :type "DamageType Object Reference") (InstigatedBy :type "Controller Object Reference") (DamageCauser :type "Actor Object Reference"))
  ;[1 1 1] Receiving damage
  (if (not (`self.bInvincible`))
    ;;[1 1 1] Check if already dead
    (if (> (`self.CurrentHealth`) 0.0)
      (bind _output_get (set `self.CurrentHealth` (`KismetMathLibrary.FClamp` (- (`self.CurrentHealth`) Damage) 0.0 (`self.MaxHealth`))))
      (if (<= _output_get 0.0)
        (`self.Die`)))))

(event `self.ReceiveBeginPlay`
  (`self.Setup Weapons` 0))

(event `self.ReceiveTick`
  (params (DeltaSeconds :type "Float (single-precision)")))

(event `OnStun`
  (params (Duration :type "Float (double-precision)"))
  (if (not (`self.bStunned`))
    (bind _output_get (set `self.AiController` (`AIBlueprintHelperLibrary.GetAIController` self)))
    (`Controller.UnPossess` _output_get)
    (`KismetSystemLibrary.K2_SetTimerDelegate` (delegate `OnUnStun`) Duration)
    (set `self.bStunned` true)))

(event `OnUnStun`
  (`Controller.Possess` (`self.AiController`) self)
  (set `self.bStunned` false))

(fn `ChangeWeapon`
  (params (WeaponNum :type Integer))
  (if (and (!= WeaponNum (`self.CurrentWeaponNum`)) (not (`self.bAttacking`)))
    (`/Game/MicroDoom/Weapons/BP_BaseWeapon.SetWeaponActive` (`self.GetCurrentWeapon`) false)
    (set `self.CurrentWeaponNum` WeaponNum)
    (`/Game/MicroDoom/Weapons/BP_BaseWeapon.SetWeaponActive` (`self.GetCurrentWeapon`) true)))

(fn `Die`
  (locals (TmpDestructionCounter :type Integer))
  (bind _outactors (`self.GetAttachedActors` true))
  ;[1 1 1] Destroy actor and all weapons
  ;;[1 1 1] Use reversed loop since otherwise after destroying 1 element array will change and loop will stop
  (bind _output_get (set `local.TmpDestructionCounter` (`KismetArrayLibrary.Array_Length` _outactors)))
  (while (> _output_get 0)
    (bind _result (`/Engine/EditorBlueprintResources/StandardMacros.DecrementInt` (`local.TmpDestructionCounter`))
      (:`  `
        (`self.K2_DestroyActor` (`|GetArrayItem` _outactors _result)))))
  (`self.K2_DestroyActor`))

(fn `GetCurrentHealthFraction`
  (returns (Fraction :type "Float (double-precision)"))
  (return (/ (`self.CurrentHealth`) (`self.MaxHealth`))))

(fn `GetCurrentWeapon`
  (returns (Weapon :type "/Game/MicroDoom/Weapons/BP_BaseWeapon Object Reference"))
  (return (`|GetArrayItem` (`self.WeaponInstances`) (`self.CurrentWeaponNum`))))

(fn `Push`
  (params (Direction :type "Vector Structure") (power :type "Float (double-precision)"))
  (`self.OnStun` 1.5)
  (`CharacterMovementComponent.AddImpulse` (`self.CharacterMovement`) (* Direction power) true))

(fn `Setup Weapons`
  (params (StartingWeaponNum :type Integer))
  (bind (_returnvalue_location _returnvalue_rotation) (`KismetMathLibrary.BreakTransform` (`self.GetTransform`)))
  (bind _weaponinstances (`self.WeaponInstances`))
  (for _array_element (`self.WeaponClasses`)
    ;[1 1 1] spawn all weapon and deactivate
    (if (`KismetSystemLibrary.IsValidClass` _array_element)
      (bind _returnvalue (`|SpawnActorFromClass` _array_element (`KismetMathLibrary.MakeTransform` _returnvalue_location _returnvalue_rotation) "Undefined" "OverrideRootScale" self null))
      (set `/Game/MicroDoom/Weapons/BP_BaseWeapon.CharacterOwner` self _returnvalue)
      (`KismetArrayLibrary.Array_Add` (`self.WeaponInstances`) _returnvalue)
      (`/Game/MicroDoom/Weapons/BP_BaseWeapon.SetWeaponActive` _returnvalue false)
      (`self.K2_AttachToComponent` _returnvalue (`self.Mesh`) (`/Game/MicroDoom/Weapons/BP_BaseWeapon.SocketToAttach` _returnvalue) "SnapToTarget" "SnapToTarget" "KeepRelative" true)))
  ;[1 1 1] Set current weapon
  (if (> (`KismetArrayLibrary.Array_Length` _weaponinstances) 0)
    (`/Game/MicroDoom/Weapons/BP_BaseWeapon.SetWeaponActive` (`|GetArrayItem` _weaponinstances StartingWeaponNum) true)
    (set `self.CurrentWeaponNum` StartingWeaponNum)))

(fn `UserConstructionScript`)