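; Weapon pickup collectable in MicroDoom that gives the hero the weapon set by its WeaponClass.
; It overrides OnTouch, calls the parent version, then casts the toucher to BP_Hero.
; The hero's GetWeapon result for that class is passed to ChangeWeapon to switch weapons.
; It returns true for a hero and false for any other actor.
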(fn `OnTouch`
  (params (Who :type "Actor Object Reference"))
  (returns (bWasColected :type Boolean))
  (`parent.OnTouch` Who)
  (bind _asbp_hero (cast `/Game/MicroDoom/Characters/Hero/BP_Hero` Who)
    (:`then`
      (bind _newweaponnum (`/Game/MicroDoom/Characters/BP_BaseCharacter.GetWeapon` _asbp_hero (`self.WeaponClass`)))
      (`/Game/MicroDoom/Characters/BP_BaseCharacter.ChangeWeapon` _asbp_hero _newweaponnum)
      (return true))
    (:`CastFailed`
      (return false))))

(fn `UserConstructionScript`
  (`parent.UserConstructionScript`))