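; BP_HealCollectable is a collectable pickup that heals whoever touches it.
; It overrides OnTouch, runs the parent check first, then uses BPI_Healable to ask whether the toucher needs healing.
; If so, it sends HealAmount through HealMessage and returns true; otherwise it returns false.
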(fn `OnTouch`
  (params (Who :type "Actor Object Reference"))
  (returns (bWasColected :type Boolean))
  (bind _bwascolected (`parent.OnTouch` Who))
  (if _bwascolected
    (if (`KismetSystemLibrary.DoesImplementInterface` Who "/Game/MicroDoom/Util/BPI_Healable.BPI_Healable_C")
      (bind _doneed (message `/Game/MicroDoom/Util/BPI_Healable.NeedHealing` Who))
      (if _doneed
        (message `/Game/MicroDoom/Util/BPI_Healable.Heal` Who (`self.HealAmount`))
        (return true)
        (else
          _))))
  (return false))

(fn `UserConstructionScript`
  (`parent.UserConstructionScript`))