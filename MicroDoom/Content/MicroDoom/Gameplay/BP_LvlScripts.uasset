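; BP_LvlScripts is a level-flow actor that runs a checkpointed wave encounter when the Hero enters its trigger volume.
; On the first overlap it stores the player start tag and NeedToHave in MainGameInstance, then starts the WavesSpawner.
; When all waves finish it opens the Gates, and if the player pawn is destroyed after triggering, it reloads the current level.
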(event `self.TriggerVolume.OnComponentBeginOverlap`
  (params (OverlappedComponent :type "PrimitiveComponent Object Reference") (OtherActor :type "Actor Object Reference") (OtherComp :type "PrimitiveComponent Object Reference") (OtherBodyIndex :type Integer) (bFromSweep :type Boolean) (SweepResult :type "HitResult Structure (by ref)"))
  (bind _wavesspawner (`self.WavesSpawner`))
  (if (`self.ActorHasTag` OtherActor "Hero")
    (`/Engine/EditorBlueprintResources/StandardMacros.DoOnce` false
      (:`Completed`
        ;[1 1 1] Set checkpoint
        (bind _asmain_game_instance (cast `/Game/MicroDoom/Gameplay/MainGameInstance` (`GameplayStatics.GetGameInstance`)))
        (set `/Game/MicroDoom/Gameplay/MainGameInstance.CurrentPlayerStartTag` (`KismetStringLibrary.Conv_NameToString` (`PlayerStart.PlayerStartTag` (`self.PlayerStart`))) _asmain_game_instance)
        (set `/Game/MicroDoom/Gameplay/MainGameInstance.NeedToHave` (`self.NeedToHave`) _asmain_game_instance)
        (`/Game/MicroDoom/Gameplay/BP_SpawnManager.StartSpawnManager` _wavesspawner)
        (add `/Game/MicroDoom/Gameplay/BP_SpawnManager.OnAllWavesFinished` _wavesspawner (delegate `OpenTheGates`))
        (add `self.OnDestroyed` (`GameplayStatics.GetPlayerPawn` 0) (delegate `RespawnPlayer`))))))

(event `OpenTheGates`
  (`/Game/MicroDoom/Characters/Objects/BP_Gates.Open` (`self.Gates`)))

(event `RespawnPlayer` :!signature `self.OnDestroyed`
  (params (DestroyedActor :type "Actor Object Reference"))
  (bind _returnvalue (`GameplayStatics.GetCurrentLevelName` true))
  (`GameplayStatics.OpenLevel` (`KismetStringLibrary.Conv_StringToName` _returnvalue)))

(event `self.ReceiveBeginPlay`)

(fn `UserConstructionScript`)