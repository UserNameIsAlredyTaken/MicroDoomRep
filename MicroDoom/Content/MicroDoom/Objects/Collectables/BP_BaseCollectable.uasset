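; BP_BaseCollectable is the base Blueprint for collectables in MicroDoom that are picked up on overlap.
; When its Sphere is overlapped, it asks OnTouch whether the touch counts; this base version accepts any actor, leaving a hook for children to override.
; On success it spawns a scaled particle effect, plays an optional sound, calls the OnCollect dispatcher and destroys itself.
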(event `self.Sphere.OnComponentBeginOverlap`
  (params (OverlappedComponent :type "PrimitiveComponent Object Reference") (OtherActor :type "Actor Object Reference") (OtherComp :type "PrimitiveComponent Object Reference") (OtherBodyIndex :type Integer) (bFromSweep :type Boolean) (SweepResult :type "HitResult Structure (by ref)"))
  (bind _particlesscale (`self.ParticlesScale`))
  (bind _collectsound (`self.CollectSound`))
  (bind _bwascolected (`self.OnTouch` OtherActor))
  (if _bwascolected
    ;[1 1 1] Spawn FX
    (`GameplayStatics.SpawnEmitterAtLocation` (`self.Particles`) (`SceneComponent.K2_GetComponentLocation` (`self.Sphere`)) (struct :`Yaw` 1.0) (`KismetMathLibrary.MakeVector` _particlesscale _particlesscale _particlesscale))
    ;[1 1 1] Play sound
    (`/Engine/EditorBlueprintResources/StandardMacros.IsValid` _collectsound
      (:`Is Valid`
        (`GameplayStatics.PlaySoundAtLocation` _collectsound (`self.K2_GetActorLocation`) (struct) 1.0 1.0 0.0 null null null))
      (:`Is Not Valid`
        _))
    (`self.OnCollect`)
    (`self.K2_DestroyActor`)))

(fn `OnTouch`
  (params (Who :type "Actor Object Reference"))
  (returns (bWasColected :type Boolean))
  (return true))

(fn `UserConstructionScript`)