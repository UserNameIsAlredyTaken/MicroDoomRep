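; BP_Gates is a gate actor for MicroDoom that slides open when its Open event is called.
; Open stores the current location, then plays a timeline whose Shift track, scaled by OpenSpeed, offsets the gate along the normalized OpenDirection.
; Each update teleports the actor without sweep, and the Blueprint contains no closing logic.
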(event `Open`
  (set `self.OldLocation` (`self.K2_GetActorLocation`))
  (bind (_direction _shift) (`Timeline|Timeline_0`)
    (:`Update`
      (`self.K2_SetActorLocation` (+ (* (`KismetMathLibrary.Normal` (`self.OpenDirection`)) (* _shift (`self.OpenSpeed`))) (`self.OldLocation`)) false true))))

(fn `UserConstructionScript`)