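; A MicroDoom gate actor that slides away from its position when its Open event is called.
; Open plays the opening sound at the gate, stores the current location, then runs a timeline that teleports the gate along the normalized OpenDirection, with the timeline's Shift curve scaled by OpenSpeed as the distance.
; The whole opening, movement included, runs only if OpeningSound is valid.
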(event `Open`
  (bind _openingsound (`self.OpeningSound`))
  (`/Engine/EditorBlueprintResources/StandardMacros.IsValid` _openingsound
    (:`Is Valid`
      (`GameplayStatics.PlaySoundAtLocation` _openingsound (`self.K2_GetActorLocation`) (struct) 1.0 1.0 0.0 null null null)
      (set `self.OldLocation` (`self.K2_GetActorLocation`))
      (bind (_direction _shift) (`Timeline|Timeline_0`)
        (:`Update`
          (`self.K2_SetActorLocation` (+ (* (`KismetMathLibrary.Normal` (`self.OpenDirection`)) (* _shift (`self.OpenSpeed`))) (`self.OldLocation`)) false true))))))

(fn `UserConstructionScript`)