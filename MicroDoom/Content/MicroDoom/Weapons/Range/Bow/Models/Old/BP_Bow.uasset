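; Bow weapon with a charged shot and a cone knockback special.
; Montage notifies time the draw and release, with pull time driving a Niagara aim beam's color and the damage curve; arrows home on the hero's last aim target.
; The special pushes enemies toward nearby "PushTarget" actors, harder if stunned, with brief slow-motion.
; Berserk swaps the damage and color curves, and damage dealt updates the special's cooldown.
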(event `self.ReceiveTick`
  (params (DeltaSeconds :type "Float (single-precision)"))
  (`parent.ReceiveTick` DeltaSeconds)
  (if (`self.bPulling`)
    ;[1 1 1] Count how long pulling string
    (set `self.PullingTime` (+ (`self.PullingTime`) (`GameplayStatics.GetWorldDeltaSeconds`)))
    ;[1 1 1] Update Beam
    (`NiagaraComponent.SetVariableLinearColor` (`self.NiagaraBeam`) "Color" (`CurveLinearColor.GetLinearColorValue` (`self.ColorCurve`) (`self.PullingTime`)))
    (`NiagaraComponent.SetVariableVec3` (`self.NiagaraBeam`) "Beam End" (+ (`SceneComponent.K2_GetComponentLocation` (`self.ShootPoint`)) (* (`SceneComponent.GetForwardVector` (`Actor.RootComponent` (`self.GetOwner`))) (`self.Range`))))))

(event `/Game/MicroDoom/Util/BPI_HeroWeapon.BercerkOn`
  (set `self.SavedDmgCurve` (`self.DamageCurve`))
  (set `self.DamageCurve` (`self.BercerkDmgCurve`))
  (set `self.SavedColorCurve` (`self.ColorCurve`))
  (set `self.ColorCurve` (`self.BercerkColorCurve`)))

(event `/Game/MicroDoom/Util/BPI_HeroWeapon.BercerkOff`
  (set `self.DamageCurve` (`self.SavedDmgCurve`))
  (set `self.ColorCurve` (`self.SavedColorCurve`)))

(event `/Game/MicroDoom/Util/BPI_HeroWeapon.HandleDmg`
  (params (WhoWasDamaged :type "/Game/MicroDoom/Characters/BP_BaseCharacter Object Reference") (Dmg :type "Float (single-precision)"))
  ;[1 1 1] Update cooldpwn on damaging enemies
  (`self.UpdateSpecialCooldown` Dmg))

(event `BowSpecial`
  (bind _returnvalue (/ (`self.PushDetectionRadius`) 200.0))
  (bind _returnvalue_2 (- (`SceneComponent.K2_GetComponentLocation` (`Actor.RootComponent` (`self.PushedActor`))) (`SceneComponent.K2_GetComponentLocation` (`Actor.RootComponent` (`self.CharacterOwner`)))))
  (if (not (`self.bSpecialInProgress`))
    (`self.StartSpecial`)
    (`|PlayMontage` (`Character.Mesh` (`self.CharacterOwner`)) (`self.SkillAnimMontage`) 1.0 0.0 "Default"
      (:`OnCompleted`
        (`self.FinishSpecial` :!label _label))
      (:`OnInterrupted`
        (goto _label))
      (:`OnNotifyBegin`
        (bind _enemies (`/Game/MicroDoom/Util/ConeDetectionUtil.GetAllEnemiesInCone` (`self.CharacterOwner`) (`self.PushDetectionRadius`) (`self.PushDetectionAngles`)))
        (for _array_element _enemies
          (set `self.PushedActor` _array_element)
          (bind _closesttarget (`/Game/MicroDoom/Util/ConeDetectionUtil.FindTargetInCone` (`KismetMathLibrary.Conv_VectorToRotator` _returnvalue_2) (`self.PushTargetDetectionAngels`) "PushTarget" (`self.PushedActor`) (`self.PushTargetDetectionRadius`)))
          (`/Engine/EditorBlueprintResources/StandardMacros.IsValid` _closesttarget
            (:`Is Valid`
              (set `self.PushDirection` (- (`SceneComponent.K2_GetComponentLocation` (`Actor.RootComponent` _closesttarget)) (`SceneComponent.K2_GetComponentLocation` (`Actor.RootComponent` (`self.PushedActor`))))))
            (:`Is Not Valid`
              (set `self.PushDirection` _returnvalue_2)))
          (`/Game/MicroDoom/Characters/BP_BaseCharacter.Push` (`self.PushedActor`) (`KismetMathLibrary.Normal` (`self.PushDirection`)) (* (`self.PushPower`) (`KismetMathLibrary.SelectFloat` (`self.StunnedPushMultiplier`) 1.0 (`/Game/MicroDoom/Characters/BP_BaseCharacter.bStunned` (`self.PushedActor`)))))
          (`GameplayStatics.SetGlobalTimeDilation` 0.5)
          (`KismetSystemLibrary.Delay` 0.05)
          (`GameplayStatics.SetGlobalTimeDilation` 1.0))
        ;[1 1 1] Spawn FX
        (`GameplayStatics.SpawnEmitterAtLocation` "/Game/MicroDoom/Weapons/Range/Bow/P_RBurst_Fire_Charge_01.P_RBurst_Fire_Charge_01" (`SceneComponent.K2_GetComponentLocation` (`Character.CapsuleComponent` (`self.CharacterOwner`))) (struct) (`KismetMathLibrary.MakeVector` _returnvalue _returnvalue _returnvalue))
        (`self.SetCooldown` true)))))

(event `BowMain`
  (`self.StartMainAttack`)
  (`|PlayMontage` (`Character.Mesh` (`self.CharacterOwner`)) (`self.AttackAnimMontage`) 1.0 0.0 "DrawArrow"
    (:`OnCompleted`
      (`self.FinishMainAttack` :!label _label))
    (:`OnInterrupted`
      (goto _label))
    (:`OnNotifyBegin`
      (`self.ToggleNotifyPeriod` true))
    (:`OnNotifyEnd`
      (`self.ToggleNotifyPeriod` false))))

(event `BowRelease`
  (`AnimInstance.Montage_SetNextSection` (`SkeletalMeshComponent.GetAnimInstance` (`Character.Mesh` (`self.CharacterOwner`))) "Hold" "None" (`self.AttackAnimMontage`)))

(fn `AttackRelease`
  (`self.BowRelease`))

(fn `CallMainAttack`
  (params (AttackTarget :type "Actor Object Reference"))
  (`self.BowMain`))

(fn `CallSpecial`
  (returns (bOnCooldown :type Boolean))
  (bind _boncooldown (`parent.CallSpecial`))
  (if (not _boncooldown)
    (`self.BowSpecial`))
  (return _boncooldown))

(fn `FinishMainAttack`
  (`parent.FinishMainAttack`)
  (set `/Game/MicroDoom/Characters/BP_BaseCharacter.bMoving` true (`self.CharacterOwner`)))

(fn `GetUI`
  (returns (WeaponUI :type "UserWidget Class Reference"))
  (return "/Game/MicroDoom/UI/WeaponWidgets/BowWidget.BowWidget_C"))

(fn `InterruptAction`
  (`Character.StopAnimMontage` (`self.CharacterOwner`) null)
  (set `self.bPulling` false)
  (set `self.PullingTime` 0.0)
  (`SceneComponent.SetVisibility` (`self.NiagaraBeam`) false false))

(fn `Shoot`
  (params (Damage :type "Float (double-precision)") (ShootTarget :type "Actor Object Reference"))
  (returns (ShootedProjectileMovement :type "ProjectileMovementComponent Object Reference"))
  (bind _shootedprojectilemovement (`parent.Shoot` (* (`self.Damage`) (`CurveFloat.GetFloatValue` (`self.DamageCurve`) (`self.PullingTime`))) null))
  (`/Engine/EditorBlueprintResources/StandardMacros.IsValid` _shootedprojectilemovement
    (:`Is Valid`
      (bind _asbp_hero (cast `/Game/MicroDoom/Characters/Hero/BP_Hero` (`self.CharacterOwner`)))
      (bind _lastaimtarget (`/Game/MicroDoom/Characters/Hero/BP_Hero.LastAimTarget` _asbp_hero))
      (`/Engine/EditorBlueprintResources/StandardMacros.IsValid` _lastaimtarget
        (:`Is Valid`
          (set `ProjectileMovementComponent.HomingTargetComponent` (`Actor.RootComponent` _lastaimtarget) _shootedprojectilemovement)
          (return _shootedprojectilemovement))))))

(fn `StartMainAttack`
  (`parent.StartMainAttack`)
  (set `/Game/MicroDoom/Characters/BP_BaseCharacter.bMoving` false (`self.CharacterOwner`)))

(fn `ToggleNotifyPeriod`
  (params (bStart :type Boolean))
  (`parent.ToggleNotifyPeriod` bStart)
  (if bStart
    (set `self.bPulling` true)
    (`SceneComponent.SetVisibility` (`self.NiagaraBeam`) true false)
    (else
      (set `self.bPulling` false)
      (`self.Shoot` 0.0)
      (set `self.PullingTime` 0.0)
      (`SceneComponent.SetVisibility` (`self.NiagaraBeam`) false false))))

(fn `UserConstructionScript`
  (`parent.UserConstructionScript`))