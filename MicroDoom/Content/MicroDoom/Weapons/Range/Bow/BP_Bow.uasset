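; Bow weapon with a charged main shot and a cooldown-gated secondary push.
; Main attack tracks draw time, driving a Niagara aim beam's color and the damage curve applied on release; projectiles home on the hero's last aim target.
; Secondary shoves enemies in a cone toward nearby "PushTarget" actors, otherwise away from the hero, with extra power against stunned ones.
; Attack notify periods start and end both attacks.
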(event `self.ReceiveTick`
  (params (DeltaSeconds :type "Float (single-precision)"))
  (`parent.ReceiveTick` DeltaSeconds)
  (if (`self.bPulling`)
    ;[1 1 1] Count how long pulling string
    (set `self.PullingTime` (+ (`self.PullingTime`) (`GameplayStatics.GetWorldDeltaSeconds`)))
    ;[1 1 1] Update Beam
    (`NiagaraComponent.SetVariableLinearColor` (`self.NiagaraBeam`) "Color" (`CurveLinearColor.GetLinearColorValue` (`self.ColorCurve`) (`self.PullingTime`)))
    (`NiagaraComponent.SetVariableVec3` (`self.NiagaraBeam`) "Beam End" (+ (`SceneComponent.K2_GetComponentLocation` (`self.ShootPoint`)) (* (`SceneComponent.GetForwardVector` (`Actor.RootComponent` (`self.GetOwner`))) 5000.0)))))

(fn `OnPushCooldownStop`)

(fn `Shoot`
  (params (Damage :type "Float (double-precision)"))
  (returns (ShootedProjectileMovement :type "ProjectileMovementComponent Object Reference"))
  (bind _shootedprojectilemovement (`parent.Shoot` (* (`self.Damage`) (`CurveFloat.GetFloatValue` (`self.DamageCurve`) (`self.PullingTime`)))))
  (`/Engine/EditorBlueprintResources/StandardMacros.IsValid` _shootedprojectilemovement
    (:`Is Valid`
      (bind _asbp_hero (cast `/Game/MicroDoom/Characters/Hero/BP_Hero` (`self.CharacterOwner`)))
      (bind _lastaimtarget (`/Game/MicroDoom/Characters/Hero/BP_Hero.LastAimTarget` _asbp_hero))
      (`/Engine/EditorBlueprintResources/StandardMacros.IsValid` _lastaimtarget
        (:`Is Valid`
          (set `ProjectileMovementComponent.HomingTargetComponent` (`Actor.RootComponent` _lastaimtarget) _shootedprojectilemovement)
          (return _shootedprojectilemovement))))))

(fn `StartAttack`
  (params (CurrentAttackType :type "/Game/MicroDoom/Weapons/AttackType Enum" :default "NewEnumerator0"))
  (switch `/Game/MicroDoom/Weapons/AttackType` CurrentAttackType
    (:`NewEnumerator0`
      (`parent.StartAttack` CurrentAttackType :!label _label))
    (:`NewEnumerator1`
      (if (== (`self.GetSecondaryCooldownFraction`) 1.0)
        (goto _label)))))

(fn `ToggleMainAttack`
  (params (Start :type Boolean))
  (if Start
    (set `self.bPulling` true)
    (`SceneComponent.SetVisibility` (`self.NiagaraBeam`) true false)
    (else
      (set `self.bPulling` false)
      (`self.Shoot` 0.0)
      (set `self.PullingTime` 0.0)
      (`SceneComponent.SetVisibility` (`self.NiagaraBeam`) false false))))

(fn `ToggleNotifyPeriod`
  (params (bStart :type Boolean))
  (`parent.ToggleNotifyPeriod` bStart)
  (switch `/Game/MicroDoom/Weapons/AttackType` (`self.CurrentAttackType`)
    (:`NewEnumerator0`
      (`self.ToggleMainAttack` bStart))
    (:`NewEnumerator1`
      (`self.ToggleSecondaryAttack` bStart)
      ;[1 1 1] Start cooldown
      (bind _returnvalue (`KismetSystemLibrary.K2_SetTimerDelegate` (`|CreateDelegate` :!event `OnPushCooldownStop`) (`self.SecondaryCooldown`)))
      (set `self.SecondaryCooldownTimer` _returnvalue))))

(fn `ToggleSecondaryAttack`
  (params (Start :type Boolean))
  (locals (PushedActor :type "/Game/MicroDoom/Characters/BP_BaseCharacter Object Reference") (PushDirection :type "Vector Structure"))
  (bind _returnvalue (- (`SceneComponent.K2_GetComponentLocation` (`Actor.RootComponent` (`local.PushedActor`))) (`SceneComponent.K2_GetComponentLocation` (`Actor.RootComponent` (`self.CharacterOwner`)))))
  (if Start
    (bind _enemies (`/Game/MicroDoom/Util/ConeDetectionUtil.GetAllEnemiesInCone` (`self.CharacterOwner`) (`self.PushinDetectionRadius`) (`self.PushDetectionAngles`)))
    (for _array_element _enemies
      (set `local.PushedActor` _array_element)
      (bind _closesttarget (`/Game/MicroDoom/Util/ConeDetectionUtil.FindTargetInCone` (`KismetMathLibrary.Conv_VectorToRotator` _returnvalue) (`self.PushTargetDetectionAngels`) "PushTarget" (`local.PushedActor`)))
      (`/Engine/EditorBlueprintResources/StandardMacros.IsValid` _closesttarget
        (:`Is Valid`
          (set `local.PushDirection` (- (`SceneComponent.K2_GetComponentLocation` (`Actor.RootComponent` _closesttarget)) (`SceneComponent.K2_GetComponentLocation` (`Actor.RootComponent` (`local.PushedActor`))))))
        (:`Is Not Valid`
          (set `local.PushDirection` _returnvalue)))
      (`/Game/MicroDoom/Characters/BP_BaseCharacter.Push` (`local.PushedActor`) (`KismetMathLibrary.Normal` (`local.PushDirection`)) (* (`self.PushPower`) (`KismetMathLibrary.SelectFloat` (`self.StunnedPushMultiplier`) 1.0 (`/Game/MicroDoom/Characters/BP_BaseCharacter.bStunned` (`local.PushedActor`))))))))

(fn `UserConstructionScript`
  (`parent.UserConstructionScript`))