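; Base ranged weapon Blueprint for MicroDoom that fires projectiles and can switch on auto-aim for the hero wielding it.
; Shoot spawns the projectile at ShootPoint, passes it damage and ally tag, launches it along the owner's forward vector and returns its movement component.
; When AutoAim is set, CallMainAttack enables auto-aiming on BP_Hero with the weapon's angle setting, and FinishAttack disables it.
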(fn `CallMainAttack`
  (bind _characterowner (`self.CharacterOwner`))
  (`parent.CallMainAttack`)
  (if (`self.bAutoAim`)
    (`/Engine/EditorBlueprintResources/StandardMacros.IsValid` _characterowner
      (:`Is Valid`
        (bind _asbp_hero (cast `/Game/MicroDoom/Characters/Hero/BP_Hero` _characterowner))
        (set `/Game/MicroDoom/Characters/Hero/BP_Hero.bAutoAiming` true _asbp_hero)
        (set `/Game/MicroDoom/Characters/Hero/BP_Hero.AutoAimingDegrees` (`self.AutoAimDegrees`) _asbp_hero)))))

(fn `FinishAttack`
  (bind _characterowner (`self.CharacterOwner`))
  (`parent.FinishAttack`)
  (if (`self.bAutoAim`)
    (`/Engine/EditorBlueprintResources/StandardMacros.IsValid` _characterowner
      (:`Is Valid`
        (bind _asbp_hero (cast `/Game/MicroDoom/Characters/Hero/BP_Hero` _characterowner))
        (set `/Game/MicroDoom/Characters/Hero/BP_Hero.bAutoAiming` false _asbp_hero)))))

(fn `Shoot`
  (params (Damage :type "Float (double-precision)"))
  (returns (ShootedProjectileMovement :type "ProjectileMovementComponent Object Reference"))
  (bind _returnvalue (`|SpawnActorFromClass` (`self.Projectile`) (`SceneComponent.K2_GetComponentToWorld` (`self.ShootPoint`)) "Undefined" "OverrideRootScale" self null))
  (`/Engine/EditorBlueprintResources/StandardMacros.IsValid` _returnvalue
    (:`Is Valid`
      (set `/Game/MicroDoom/Weapons/Range/BP_BaseProjectile.Damage` Damage _returnvalue)
      (set `/Game/MicroDoom/Weapons/Range/BP_BaseProjectile.AllyTag` (`self.AllyTag`) _returnvalue)
      (bind _projectilemovement (`/Game/MicroDoom/Weapons/Range/BP_BaseProjectile.ProjectileMovement` _returnvalue))
      (set `ProjectileMovementComponent.MaxSpeed` (`self.Speed`) _projectilemovement)
      (set `MovementComponent.Velocity` (* (`SceneComponent.GetForwardVector` (`Actor.RootComponent` (`self.GetOwner`))) (`self.Speed`)) _projectilemovement)
      (return _projectilemovement))))

(fn `UserConstructionScript`
  (`parent.UserConstructionScript`))