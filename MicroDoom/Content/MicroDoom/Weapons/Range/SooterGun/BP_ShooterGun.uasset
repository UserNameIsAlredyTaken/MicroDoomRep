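; BP_ShooterGun is a ranged weapon Blueprint in MicroDoom that fires repeatedly while its main attack is active.
; CallMainAttack runs the parent logic, then starts a looping timer spaced by ShotsDelay, and FinishMainAttack clears that timer.
; CallShootWithParameters passes the gun's Damage to Shoot, while the event graph holds only disabled default events.
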(fn `CallMainAttack`
  (`parent.CallMainAttack`)
  (bind _returnvalue (`KismetSystemLibrary.K2_SetTimerDelegate` (`|CreateDelegate` :!event `CallShootWithParameters`) (`self.ShotsDelay`) true))
  (set `self.ShootTimer` _returnvalue))

(fn `CallShootWithParameters`
  (`self.Shoot` (`self.Damage`)))

(fn `FinishMainAttack`
  (`parent.FinishMainAttack`)
  (`KismetSystemLibrary.K2_ClearAndInvalidateTimerHandle` (`self.ShootTimer`)))

(fn `UserConstructionScript`
  (`parent.UserConstructionScript`))