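; BP_BaseProjectile is the base projectile for MicroDoom's ranged weapons, dealing damage on contact.
; When its Collider begins an overlap, it ignores actors tagged Projectile, actors carrying its AllyTag, and its own owner.
; Any other actor receives the projectile's Damage through ApplyDamage, and the projectile then destroys itself.
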(event `self.Collider.OnComponentBeginOverlap`
  (params (OverlappedComponent :type "PrimitiveComponent Object Reference") (OtherActor :type "Actor Object Reference") (OtherComp :type "PrimitiveComponent Object Reference") (OtherBodyIndex :type Integer) (bFromSweep :type Boolean) (SweepResult :type "HitResult Structure (by ref)"))
  (if (and (not (`self.ActorHasTag` OtherActor "Projectile")) (not (`self.ActorHasTag` OtherActor (`self.AllyTag`))) (not (== OtherActor (`self.GetOwner`))))
    (`GameplayStatics.ApplyDamage` OtherActor (`self.Damage`))
    (`self.K2_DestroyActor`)))

(fn `UserConstructionScript`)