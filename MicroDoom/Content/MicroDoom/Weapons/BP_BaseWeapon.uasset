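; Base weapon Blueprint for MicroDoom that provides shared attack state and activation logic.
; StartAttack stores the attack type and sets the owning character's Attacking flag, while FinishAttack clears it and calls a finish-attack event.
; ToggleNotifyPeriod is an empty hook for animation notify windows, such as bow draws or melee damage sweeps, with only disconnected debug prints.
; SetWeaponActive toggles visibility, collision and tick together.
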(fn `FinishAttack`
  (bind _characterowner (`self.CharacterOwner`))
  (`/Engine/EditorBlueprintResources/StandardMacros.IsValid` _characterowner
    (:`Is Valid`
      (set `/Game/MicroDoom/Characters/BP_BaseCharacter.bAttacking` false _characterowner)
      (`self.FinishAttackEvent`))))

(fn `SetWeaponActive`
  (params (bActive :type Boolean))
  (`self.SetActorHiddenInGame` (not bActive))
  (`self.SetActorEnableCollision` bActive)
  (`self.SetActorTickEnabled` bActive))

(fn `StartAttack`
  (params (CurrentAttackType :type "/Game/MicroDoom/Weapons/AttackType Enum" :default "NewEnumerator0"))
  (bind _characterowner (`self.CharacterOwner`))
  (set `self.CurrentAttackType` CurrentAttackType)
  (`/Engine/EditorBlueprintResources/StandardMacros.IsValid` _characterowner
    (:`Is Valid`
      (set `/Game/MicroDoom/Characters/BP_BaseCharacter.bAttacking` true _characterowner))))

(fn `ToggleNotifyPeriod`
  (params (bStart :type Boolean))
  ;[1 1 1] Start o finish notifing period of animation for weapon
  ; For bows it is period of pulling string
  ; For mele it is period of damaging sweep
)

(fn `UserConstructionScript`)