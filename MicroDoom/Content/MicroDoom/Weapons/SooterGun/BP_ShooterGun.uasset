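; BP_ShooterGun is a MicroDoom weapon that fires enemy projectiles at a fixed interval while an attack is active.
; StartAttack calls the parent, then starts a looping timer on Shoot using ShotsDelay, so the first shot comes after one delay.
; Shoot spawns a BP_EnemyProjectile at the ShootPoint transform with a limited lifespan.
; FinishAttack calls the parent, then clears the timer to stop firing.
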(event `self.ReceiveTick`
  (params (DeltaSeconds :type "Float (single-precision)"))
  (`parent.ReceiveTick` DeltaSeconds))

(fn `FinishAttack`
  (`parent.FinishAttack`)
  (`KismetSystemLibrary.K2_ClearAndInvalidateTimerHandle` (`self.ShootTimer`)))

(fn `Shoot`
  (bind _returnvalue (`|SpawnActorFromClass` "/Game/MicroDoom/Weapons/SooterGun/BP_EnemyProjectile.BP_EnemyProjectile_C" (`SceneComponent.K2_GetComponentToWorld` (`self.ShootPoint`)) "Undefined" "OverrideRootScale" null null))
  (`self.SetLifeSpan` _returnvalue 10.0))

(fn `StartAttack`
  (`parent.StartAttack`)
  (bind _returnvalue (`KismetSystemLibrary.K2_SetTimer` null "Shoot" (`self.ShotsDelay`) true))
  (set `self.ShootTimer` _returnvalue))

(fn `UserConstructionScript`
  (`parent.UserConstructionScript`))