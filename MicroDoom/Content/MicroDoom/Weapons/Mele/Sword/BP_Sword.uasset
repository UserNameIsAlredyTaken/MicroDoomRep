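; BP_Sword is a melee weapon with a four-hit combo and a cone stun special.
; Attacks pressed mid-swing are buffered for the next montage, whose notifies toggle hit windows and trails, while walk speed is scaled during attacks.
; The special resets the combo, damages and stuns enemies in a radius-scaled burst, and its cooldown updates from damage dealt.
; Berserk events swap the trail and multiply attack speed and damage, then revert them.
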(event `/Game/MicroDoom/Util/BPI_HeroWeapon.HandleDmg`
  (params (WhoWasDamaged :type "/Game/MicroDoom/Characters/BP_BaseCharacter Object Reference") (Dmg :type "Float (single-precision)"))
  ;[1 1 1] Update cooldpwn on damaging enemies
  (`self.UpdateSpecialCooldown` Dmg))

(event `self.ReceiveTick`
  (params (DeltaSeconds :type "Float (single-precision)"))
  (`parent.ReceiveTick` DeltaSeconds))

(event `/Game/MicroDoom/Util/BPI_HeroWeapon.BercerkOn`
  ;[1 1 1] Save old trail
  (set `self.SavedTrail` (`ParticleSystemComponent.Template` (`self.Trail`)))
  ;[1 1 1] Set berserk trail
  (`ParticleSystemComponent.SetTemplate` (`self.Trail`) (`self.BercerkTrail`))
  ;[1 1 1] Set new attack speed
  (set `self.AttackSpeed` (* (`self.AttackSpeed`) (`self.BercerkAttackSpeedMul`)))
  ;[1 1 1] Set new damage
  (set `self.Damage` (* (`self.Damage`) (`self.BercerkDmgMul`))))

(event `/Game/MicroDoom/Util/BPI_HeroWeapon.BercerkOff`
  ;[1 1 1] Reset trail
  (`ParticleSystemComponent.SetTemplate` (`self.Trail`) (`self.SavedTrail`))
  ;[1 1 1] Reset attack speed
  (set `self.AttackSpeed` (/ (`self.AttackSpeed`) (`self.BercerkAttackSpeedMul`)))
  ;[1 1 1] Reset damage
  (set `self.Damage` (/ (`self.Damage`) (`self.BercerkDmgMul`))))

(event `SwordAttack`
  (if (`/Game/MicroDoom/Characters/BP_BaseCharacter.bAttacking` (`self.CharacterOwner`))
    (set `self.SaveAttack` true)
    (else
      (`self.StartMainAttack`)
      (switch `int` (`self.AttackCount`) :!label _label
        (:`0`
          (set `self.AttackCount` 1)
          (`|PlayMontage` (`Character.Mesh` (`self.CharacterOwner`)) "/Game/MicroDoom/Characters/Hero/Animations/Sword/Terra/Primary_Melee_A_slow_Montage.Primary_Melee_A_slow_Montage" (`self.AttackSpeed`) 0.0 "Default"
            (:`OnNotifyBegin`
              ;[1 1 1] Switch damage
              (`self.ToggleNotifyPeriod` true :!label _label_2)
              ;[1 1 1] PlayTrails
              (`ParticleSystemComponent.BeginTrails` (`self.Trail`) "FX1" "FX2" "ETrailWidthMode_FromCentre" 1.0))
            (:`OnNotifyEnd`
              (`self.ToggleNotifyPeriod` false :!label _label_3)
              (`ParticleSystemComponent.EndTrails` (`self.Trail`)))))
        (:`1`
          (set `self.AttackCount` 2)
          (`|PlayMontage` (`Character.Mesh` (`self.CharacterOwner`)) "/Game/MicroDoom/Characters/Hero/Animations/Sword/Terra/Primary_Melee_B_slow_Montage.Primary_Melee_B_slow_Montage" (`self.AttackSpeed`) 0.0 "Default"
            (:`OnNotifyBegin`
              (goto _label_2))
            (:`OnNotifyEnd`
              (goto _label_3))))
        (:`2`
          (set `self.AttackCount` 3)
          (`|PlayMontage` (`Character.Mesh` (`self.CharacterOwner`)) "/Game/MicroDoom/Characters/Hero/Animations/Sword/Terra/Primary_Melee_C_slow_Montage.Primary_Melee_C_slow_Montage" (`self.AttackSpeed`) 0.0 "Default"
            (:`OnNotifyBegin`
              (goto _label_2))
            (:`OnNotifyEnd`
              (goto _label_3))))
        (:`3`
          (set `self.AttackCount` 0)
          (`|PlayMontage` (`Character.Mesh` (`self.CharacterOwner`)) "/Game/MicroDoom/Characters/Hero/Animations/Sword/Terra/Primary_Melee_D_slow_Montage.Primary_Melee_D_slow_Montage" (`self.AttackSpeed`) 0.0 "Default"
            (:`OnNotifyBegin`
              (goto _label_2))
            (:`OnNotifyEnd`
              (goto _label_3))))))))

(event `ComboAttackSave`
  (if (`self.SaveAttack`)
    (set `self.SaveAttack` false)
    (goto _label)))

(event `ResetCombo`
  (if (`/Game/MicroDoom/Characters/BP_BaseCharacter.bAttacking` (`self.CharacterOwner`))
    (set `self.AttackCount` 0)
    (set `self.SaveAttack` false)
    (`self.FinishMainAttack`)))

(event `SwordSpecial`
  (bind _returnvalue (/ (`self.StaningDetectionRadius`) 300.0))
  (if (not (`self.bSpecialInProgress`))
    (`self.StartSpecial`)
    (`self.ResetCombo`)
    (`|PlayMontage` (`Character.Mesh` (`self.CharacterOwner`)) (`self.SkillAnimMontage`) 1.0 0.0 "Default"
      (:`OnCompleted`
        (`self.FinishSpecial` :!label _label))
      (:`OnInterrupted`
        (goto _label))
      (:`OnNotifyBegin`
        (bind _enemies (`/Game/MicroDoom/Util/ConeDetectionUtil.GetAllEnemiesInCone` (`self.CharacterOwner`) (`self.StaningDetectionRadius`) (`self.StaningDetectionAngles`)))
        (for _array_element _enemies
          (`/Game/MicroDoom/Characters/BP_BaseCharacter.Stun` _array_element (`self.StunDuration`) true)
          (`/Game/MicroDoom/Characters/BP_BaseCharacter.SwordEffect` _array_element (`self.StunDuration`))
          (`GameplayStatics.ApplyDamage` _array_element (`self.SpecialDamage`) null self))
        ;[1 1 1] Spawn FX
        (bind _returnvalue_2 (`GameplayStatics.SpawnEmitterAtLocation` "/Game/MicroDoom/Weapons/Mele/Sword/P_RBurst_Fire_Burst_Area_01.P_RBurst_Fire_Burst_Area_01" (`SceneComponent.K2_GetComponentLocation` (`Character.CapsuleComponent` (`self.CharacterOwner`)))))
        (`FXSystemComponent.SetVectorParameter` _returnvalue_2 "InstanceMeshScale" (`KismetMathLibrary.MakeVector` _returnvalue _returnvalue _returnvalue))
        (`self.SetCooldown` true)))))

(fn `CallMainAttack`
  (params (AttackTarget :type "Actor Object Reference"))
  (`self.SwordAttack`))

(fn `CallSpecial`
  (returns (bOnCooldown :type Boolean))
  (bind _boncooldown (`parent.CallSpecial`))
  (if (not _boncooldown)
    (`self.SwordSpecial`))
  (return _boncooldown))

(fn `FinishMainAttack`
  (bind _charactermovement (`Character.CharacterMovement` (`self.CharacterOwner`)))
  (`parent.FinishMainAttack`)
  (set `CharacterMovementComponent.MaxWalkSpeed` (/ (`CharacterMovementComponent.MaxWalkSpeed` _charactermovement) (`self.AttackingHeroRunSpeedMultiplier`)) _charactermovement))

(fn `GetUI`
  (returns (WeaponUI :type "UserWidget Class Reference"))
  (return "/Game/MicroDoom/UI/WeaponWidgets/AxeWidget.AxeWidget_C"))

(fn `InterruptAction`
  (`Character.StopAnimMontage` (`self.CharacterOwner`) null)
  (if (`/Game/MicroDoom/Characters/BP_BaseCharacter.bAttacking` (`self.CharacterOwner`))
    (`self.ResetCombo`)))

(fn `StartMainAttack`
  (bind _charactermovement (`Character.CharacterMovement` (`self.CharacterOwner`)))
  (`parent.StartMainAttack`)
  (set `CharacterMovementComponent.MaxWalkSpeed` (* (`CharacterMovementComponent.MaxWalkSpeed` _charactermovement) (`self.AttackingHeroRunSpeedMultiplier`)) _charactermovement))

(fn `UserConstructionScript`
  (`parent.UserConstructionScript`))