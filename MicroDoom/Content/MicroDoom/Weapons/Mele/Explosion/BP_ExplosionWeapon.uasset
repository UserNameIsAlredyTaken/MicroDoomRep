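; Proximity explosion weapon, a melee weapon Blueprint that detonates when a Hero-tagged actor enters its detection sphere.
; StartAttack damages BP_BaseCharacter pawns within the explosion radius, excluding the owner, and spawns a fire eruption scaled to that radius.
; FinishAttack then kills a BP_Barrel owner, first clearing ExplodeBeforeDeath so the death does not trigger another explosion.
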(event `self.ReceiveBeginPlay`
  (`parent.ReceiveBeginPlay`)
  (`SphereComponent.SetSphereRadius` (`self.Sphere`) (`self.DetectionRadius`) true))

(event `self.ReceiveTick`
  (params (DeltaSeconds :type "Float (single-precision)"))
  (`parent.ReceiveTick` DeltaSeconds))

(event `self.Sphere.OnComponentBeginOverlap`
  (params (OverlappedComponent :type "PrimitiveComponent Object Reference") (OtherActor :type "Actor Object Reference") (OtherComp :type "PrimitiveComponent Object Reference") (OtherBodyIndex :type Integer) (bFromSweep :type Boolean) (SweepResult :type "HitResult Structure (by ref)"))
  (`/Engine/EditorBlueprintResources/StandardMacros.IsValid` OtherActor
    (:`Is Valid`
      (if (`self.ActorHasTag` OtherActor "Hero")
        (`self.StartAttack` "NewEnumerator0")
        (`self.FinishAttack`)))))

(fn `FinishAttack`
  (`parent.FinishAttack`)
  (bind _asbp_barrel (cast `/Game/MicroDoom/Characters/Enemies/Barrel/BP_barrel` (`self.GetOwner`)))
  ;[1 1 1] If callling death because of self explosion, do not explode becouse of death
  (set `/Game/MicroDoom/Characters/Enemies/Barrel/BP_barrel.ExplodeBeforeDeath` false _asbp_barrel)
  (`/Game/MicroDoom/Characters/BP_BaseCharacter.Die` _asbp_barrel))

(fn `StartAttack`
  (params (CurrentAttackType :type "/Game/MicroDoom/Weapons/AttackType Enum" :default "NewEnumerator0"))
  (locals (BaseFxRadius :type "Float (double-precision)" :default 250.0))
  (bind _returnvalue (/ (`self.ExplosionRadius`) (`local.BaseFxRadius`)))
  (`parent.StartAttack` CurrentAttackType)
  (bind _outactors (`KismetSystemLibrary.SphereOverlapActors` (`SceneComponent.K2_GetComponentLocation` (`self.Sphere`)) (`self.ExplosionRadius`) (`|MakeArray` "ObjectTypeQuery3" :!type "EObjectTypeQuery Enum") "/Game/MicroDoom/Characters/BP_BaseCharacter.BP_BaseCharacter_C"))
  (for _array_element _outactors
    (if (not (== _array_element (`self.GetOwner`)))
      (`GameplayStatics.ApplyDamage` _array_element (`self.Damage`))))
  ;[1 1 1] Spawn FX
  (`GameplayStatics.SpawnEmitterAtLocation` "/Game/MicroDoom/Weapons/Mele/Explosion/P_RBurst_Fire_Eruption_01.P_RBurst_Fire_Eruption_01" (`SceneComponent.K2_GetComponentLocation` (`Character.CapsuleComponent` (`self.CharacterOwner`))) (struct) (`KismetMathLibrary.MakeVector` _returnvalue _returnvalue _returnvalue)))

(fn `UserConstructionScript`
  (`parent.UserConstructionScript`))