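; Base melee weapon Blueprint that damages characters overlapping its capsule during a notify-driven damage window.
; ToggleNotifyPeriod extends the parent's version to set the Damaging flag.
; While Damaging is on, Tick polls the capsule for BP_BaseCharacter actors, skips those with AllyTag, and applies damage to the rest.
; A DamagedActors list limits each target to one hit per window and clears when the window closes.
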(event `self.ReceiveTick`
  (params (DeltaSeconds :type "Float (single-precision)"))
  (`parent.ReceiveTick` DeltaSeconds)
  ;[1 1 1] Damaging
  (if (`self.bDamaging`)
    (for _array_element (`PrimitiveComponent.GetOverlappingActors` (`self.Capsule`) "/Game/MicroDoom/Characters/BP_BaseCharacter.BP_BaseCharacter_C")
      (if (and (not (`KismetArrayLibrary.Array_Contains` (`self.DamagedActors`) _array_element)) (not (`self.ActorHasTag` _array_element (`self.AllyTag`))))
        (`GameplayStatics.ApplyDamage` _array_element (`self.Damage`))
        (`KismetArrayLibrary.Array_AddUnique` (`self.DamagedActors`) _array_element)))
    (else
      (`KismetArrayLibrary.Array_Clear` (`self.DamagedActors`)))))

(fn `ToggleNotifyPeriod`
  (params (bStart :type Boolean))
  (`parent.ToggleNotifyPeriod` bStart)
  (set `self.bDamaging` bStart))

(fn `UserConstructionScript`
  (`parent.UserConstructionScript`))