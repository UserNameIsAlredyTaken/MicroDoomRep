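; BP_Sword is a melee weapon with a main attack and a cooldown-gated secondary attack that stuns enemies.
; StartAttack passes to the parent for main attacks, and for secondary attacks only once the cooldown is complete.
; When the secondary attack's notify period starts, it starts the cooldown timer and calls Special, which stuns enemies in a cone around the owner and prints a debug string.
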(fn `OnStunCooldownStop`)

(fn `Special`
  (`KismetSystemLibrary.PrintString` "Hello")
  (bind _enemies (`/Game/MicroDoom/Util/ConeDetectionUtil.GetEnemiesInCone` (`self.CharacterOwner`) (`self.StatingDetectionRadius`) (`self.StaningDetectionAngles`)))
  (for _array_element _enemies
    (`/Game/MicroDoom/Characters/BP_BaseCharacter.OnStun` _array_element (`self.StunDuration`))))

(fn `StartAttack`
  (params (CurrentAttackType :type "/Game/MicroDoom/Weapons/AttackType Enum" :default "NewEnumerator0"))
  (switch `/Game/MicroDoom/Weapons/AttackType` CurrentAttackType
    (:`NewEnumerator0`
      (`parent.StartAttack` CurrentAttackType :!label _label))
    (:`NewEnumerator1`
      (if (== (`self.GetSecondaryCooldownFraction`) 1.0)
        (goto _label)))))

(fn `ToggleNotifyPeriod`
  (params (bStart :type Boolean))
  (switch `/Game/MicroDoom/Weapons/AttackType` (`self.CurrentAttackType`)
    (:`NewEnumerator0`
      (`parent.ToggleNotifyPeriod` bStart))
    (:`NewEnumerator1`
      (if bStart
        ;[1 1 1] Start cooldown
        (bind _returnvalue (`KismetSystemLibrary.K2_SetTimerDelegate` (`|CreateDelegate` :!event `OnStunCooldownStop`) (`self.SecondaryCooldown`)))
        (set `self.SecondaryCooldownTimer` _returnvalue)
        (`self.Special`)))))

(fn `UserConstructionScript`
  (`parent.UserConstructionScript`))