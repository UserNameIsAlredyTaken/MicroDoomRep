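; BP_ExplosionWeapon is a proximity-triggered explosion weapon that deals area damage to characters.
; Its Sphere component is sized to DetectionRadius at BeginPlay and calls StartAttack when an actor tagged Hero enters it.
; StartAttack runs the parent logic, then damages every BP_BaseCharacter pawn found within ExplosionRadius, with no team filter or ignore list.
; Tick draws debug spheres for both radii every frame.
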(event `self.ReceiveBeginPlay`
  (`parent.ReceiveBeginPlay`)
  (`SphereComponent.SetSphereRadius` (`self.Sphere`) (`self.DetectionRadius`) true))

(event `self.ReceiveTick`
  (params (DeltaSeconds :type "Float (single-precision)"))
  (bind _returnvalue (`SceneComponent.K2_GetComponentLocation` (`self.Sphere`)))
  (`parent.ReceiveTick` DeltaSeconds)
  (`KismetSystemLibrary.DrawDebugSphere` _returnvalue (`self.ExplosionRadius`) 12 (struct :`R` 1.0 :`B` 0.083156 :`A` 1.0))
  (`KismetSystemLibrary.DrawDebugSphere` _returnvalue (`self.DetectionRadius`) 12 (struct :`G` 1.0 :`B` 0.119997 :`A` 1.0)))

(event `self.Sphere.OnComponentBeginOverlap`
  (params (OverlappedComponent :type "PrimitiveComponent Object Reference") (OtherActor :type "Actor Object Reference") (OtherComp :type "PrimitiveComponent Object Reference") (OtherBodyIndex :type Integer) (bFromSweep :type Boolean) (SweepResult :type "HitResult Structure (by ref)"))
  (if (`self.ActorHasTag` OtherActor "Hero")
    (`self.StartAttack`)))

(fn `StartAttack`
  (`parent.StartAttack`)
  (bind _outactors (`KismetSystemLibrary.SphereOverlapActors` (`SceneComponent.K2_GetComponentLocation` (`self.Sphere`)) (`self.ExplosionRadius`) (`|MakeArray` "ObjectTypeQuery3" :!type "EObjectTypeQuery Enum") "/Game/MicroDoom/Characters/BP_BaseCharacter.BP_BaseCharacter_C"))
  (for _array_element _outactors
    (`GameplayStatics.ApplyDamage` _array_element (`self.Damage`))))

(fn `UserConstructionScript`
  (`parent.UserConstructionScript`))