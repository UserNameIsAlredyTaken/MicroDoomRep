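; Explosive weapon carried by a BP_Barrel character that works as a proximity bomb, detonating when the hero enters its detection sphere unless the owner is stunned.
; A looping-style ticking timeline pulses a light and plays sounds, with play rate driven by a curve over distance to the player.
; Detonation applies radius damage, scaled for enemies, spawns radius-scaled FX with shake and sound, then kills the barrel without triggering its death explosion.
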(event `self.ReceiveBeginPlay`
  (bind _tickingsound (`self.TickingSound`))
  (`|ExecutionSequence`
    (:`then_0`
      (`parent.ReceiveBeginPlay`))
    (:`then_1`
      (`SphereComponent.SetSphereRadius` (`self.Sphere`) (`self.DetectionRadius`) true))
    (:`then_2`
      (set `self.Hero` (`GameplayStatics.GetPlayerPawn` 0)))
    (:`then_3`
      ;[1 1 1] Tikking bomb
      (bind (_direction _lightintencity) (`Timeline|Tikking`)
        (:`Update`
          (`LightComponent.SetIntensity` (`self.PointLight`) (select `bool` (`/Game/MicroDoom/Characters/BP_BaseCharacter.bStunned` (`self.CharacterOwner`)) :`false` (* _lightintencity (`self.Base intensity`)))))
        (:`TikkingSound`
          (`/Engine/EditorBlueprintResources/StandardMacros.IsValid` _tickingsound
            (:`Is Valid`
              (if (not (`/Game/MicroDoom/Characters/BP_BaseCharacter.bStunned` (`self.CharacterOwner`)))
                (`GameplayStatics.PlaySoundAtLocation` _tickingsound (`self.K2_GetActorLocation`) (struct) 1.0 1.0 0.0 null null null)))))))))

(event `self.ReceiveTick`
  (params (DeltaSeconds :type "Float (single-precision)"))
  (`parent.ReceiveTick` DeltaSeconds)
  ;[1 1 1] Adjust speed of tikking
  (`TimelineComponent.SetPlayRate` (`self.Tikking`) (`CurveFloat.GetFloatValue` (`self.DistancemultiplierCurve`) (`KismetMathLibrary.Vector_Distance` (`self.K2_GetActorLocation` (`self.Hero`)) (`self.K2_GetActorLocation`)))))

(event `self.Sphere.OnComponentBeginOverlap`
  (params (OverlappedComponent :type "PrimitiveComponent Object Reference") (OtherActor :type "Actor Object Reference") (OtherComp :type "PrimitiveComponent Object Reference") (OtherBodyIndex :type Integer) (bFromSweep :type Boolean) (SweepResult :type "HitResult Structure (by ref)"))
  (`/Engine/EditorBlueprintResources/StandardMacros.IsValid` OtherActor
    (:`Is Valid`
      (if (`self.ActorHasTag` OtherActor "Hero")
        (if (not (`/Game/MicroDoom/Characters/BP_BaseCharacter.bStunned` (`self.CharacterOwner`)))
          (`self.CallMainAttack` null)
          (`self.FinishMainAttack`))))))

(fn `CallMainAttack`
  (params (AttackTarget :type "Actor Object Reference"))
  (locals (BaseFxRadius :type "Float (double-precision)" :default 230.0))
  (bind _damage (`self.Damage`))
  (bind _returnvalue (/ (`self.ExplosionRadius`) (`local.BaseFxRadius`)))
  (`parent.CallMainAttack` null)
  (bind _outactors (`KismetSystemLibrary.SphereOverlapActors` (`SceneComponent.K2_GetComponentLocation` (`self.Sphere`)) (`self.ExplosionRadius`) (`|MakeArray` "ObjectTypeQuery3" :!type "EObjectTypeQuery Enum") "/Game/MicroDoom/Characters/BP_BaseCharacter.BP_BaseCharacter_C"))
  (for _array_element _outactors
    (if (not (== _array_element (`self.GetOwner`)))
      (`GameplayStatics.ApplyDamage` _array_element (`KismetMathLibrary.SelectFloat` (* (`self.DamageToEnemyMultiplier`) _damage) _damage (`self.ActorHasTag` _array_element "Enemy")) null self)))
  ;[1 1 1] Spawn FX
  (`GameplayStatics.SpawnEmitterAtLocation` "/Game/MicroDoom/Weapons/Explosion/P_RBurst_Fire_Eruption_01.P_RBurst_Fire_Eruption_01" (`SceneComponent.GetSocketLocation` (`Character.Mesh` (`self.CharacterOwner`)) (`self.SocketToAttach`)) (struct) (`KismetMathLibrary.MakeVector` _returnvalue _returnvalue _returnvalue))
  (`PlayerCameraManager.PlayCameraShake` :`self` (`GameplayStatics.GetPlayerCameraManager` 0) :`ShakeClass` "/Game/MicroDoom/Weapons/Explosion/BP_ExplosionCamShake.BP_ExplosionCamShake_C" :`Scale` 0.3)
  (`GameplayStatics.PlaySoundAtLocation` (`self.ExpmosionSound`) (`self.K2_GetActorLocation`) (struct) 1.0 1.0 0.0 null null null))

(fn `FinishMainAttack`
  (`parent.FinishMainAttack`)
  (bind _asbp_barrel (cast `/Game/MicroDoom/Characters/Enemies/Barrel/BP_barrel` (`self.GetOwner`)))
  ;[1 1 1] If callling death because of self explosion, do not explode becouse of death
  (set `/Game/MicroDoom/Characters/Enemies/Barrel/BP_barrel.ExplodeBeforeDeath` false _asbp_barrel)
  (`/Game/MicroDoom/Characters/BP_BaseCharacter.Die` _asbp_barrel self))

(fn `UserConstructionScript`
  (`parent.UserConstructionScript`))