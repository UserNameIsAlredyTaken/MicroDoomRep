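; BP_BaseCharacter is the MicroDoom base character, providing health and weapon-based attacking.
; On BeginPlay, SetupWeapon spawns the configured weapon class, if set, and attaches it to the mesh's WeaponSocket.
; Pressing Attack sets the Attacking flag and calls Attack on the current weapon.
; AnyDamage reduces CurrentHealth, clamped between zero and MaxHealth, with no death handling in this graph.
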(event `self.ReceiveAnyDamage`
  (params (Damage :type "Float (single-precision)") (DamageType :type "DamageType Object Reference") (InstigatedBy :type "Controller Object Reference") (DamageCauser :type "Actor Object Reference"))
  ;[1 1 1] Receiving damage
  (set `self.CurrentHealth` (`KismetMathLibrary.FClamp` (- (`self.CurrentHealth`) Damage) 0.0 (`self.MaxHealth`))))

(event `self.ReceiveBeginPlay`
  ;[1 1 1] Setup
  (`self.SetupWeapon`))

(event `InputAction|Attack`
  (params (Key :type "Key Structure"))
  ;[1 1 1] Attacking
  (:`Pressed`
    (set `self.bAttacking` true)
    (`/Game/MicroDoom/Core/BP_BaseWeapon.Attack` (`self.CurrentWeapon`))))

(fn `SetupWeapon`
  (bind (_returnvalue_location _returnvalue_rotation) (`KismetMathLibrary.BreakTransform` (`self.GetTransform`)))
  ;[1 1 1] Check for null
  (if (!= (`self.WeaponToSawn`) null)
    (bind _returnvalue (`|SpawnActorFromClass` (`self.WeaponToSawn`) (`KismetMathLibrary.MakeTransform` _returnvalue_location _returnvalue_rotation) "Undefined" "OverrideRootScale" null null))
    (bind _output_get (set `self.CurrentWeapon` _returnvalue))
    (`self.K2_AttachToComponent` _output_get (`self.Mesh`) "WeaponSocket" "SnapToTarget" "SnapToTarget" "KeepRelative" true)))

(fn `UserConstructionScript`)