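; BP_EnemyBase is the base enemy Blueprint in MicroDoom, handling attack triggering and a health bar display.
; The StartAttack event passes the call on to the enemy's CurrentWeapon.
; Every Tick calls UpdateHealtBar, which casts the HealthBar component's widget to BP_EnemyHealth and sets its progress bar to current health over maximum health.
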(event `self.ReceiveTick`
  (params (DeltaSeconds :type "Float (single-precision)"))
  (`parent.ReceiveTick` DeltaSeconds)
  (`self.UpdateHealtBar`))

(event `self.StartAttack`
  (`/Game/MicroDoom/Core/BP_BaseWeapon.StartAttack` (`self.CurrentWeapon`)))

(fn `UpdateHealtBar`
  (bind _asbp_enemy_health (cast `/Game/MicroDoom/UI/BP_EnemyHealth` (`WidgetComponent.GetUserWidgetObject` (`self.HealthBar`))))
  (`ProgressBar.SetPercent` (`/Game/MicroDoom/UI/BP_EnemyHealth.ProgressBar_13` _asbp_enemy_health) (/ (`self.CurrentHealth`) (`self.MaxHealth`))))

(fn `UserConstructionScript`
  (`parent.UserConstructionScript`))